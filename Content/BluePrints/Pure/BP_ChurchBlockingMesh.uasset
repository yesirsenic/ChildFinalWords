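; BP_ChurchBlockingMesh is an actor, apparently a church blocker, that shows an on-screen text widget while the player is inside its TextColider trigger.
; On begin overlap with BP_Player, it creates WGBP_ChurchBlockingText and adds it to the viewport the first time, then reuses the cached instance by making it visible.
; On end overlap it hides the widget rather than removing it.
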(event `self.TextColider.OnComponentBeginOverlap`
  (params (OverlappedComponent :type "PrimitiveComponent Object Reference") (OtherActor :type "Actor Object Reference") (OtherComp :type "PrimitiveComponent Object Reference") (OtherBodyIndex :type Integer) (bFromSweep :type Boolean) (SweepResult :type "HitResult Structure (by ref)"))
  (cast `/Game/BluePrints/Pure/BP_Player` OtherActor)
  (if (`KismetSystemLibrary.IsValid` (`self.WGBP_ChurchBlockText`))
    (set `Widget.Visibility` "Visible" (`self.WGBP_ChurchBlockText`))
    (else
      (bind _returnvalue (`|CreateWidget` "/Game/BluePrints/Widget/WGBP_ChurchBlockingText.WGBP_ChurchBlockingText_C"))
      (`UserWidget.AddToViewport` _returnvalue 0)
      (set `self.WGBP_ChurchBlockText` _returnvalue))))

(event `self.TextColider.OnComponentEndOverlap`
  (params (OverlappedComponent :type "PrimitiveComponent Object Reference") (OtherActor :type "Actor Object Reference") (OtherComp :type "PrimitiveComponent Object Reference") (OtherBodyIndex :type Integer))
  (bind _wgbp_churchblocktext (`self.WGBP_ChurchBlockText`))
  (cast `/Game/BluePrints/Pure/BP_Player` OtherActor)
  (if (`KismetSystemLibrary.IsValid` _wgbp_churchblocktext)
    (set `Widget.Visibility` "Hidden" _wgbp_churchblocktext)))

(fn `UserConstructionScript`)