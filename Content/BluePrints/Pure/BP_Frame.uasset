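; BP_Frame is a picture frame with a flickering bulb whose portrait switches between a girl and a ghost.
; A looping timer, its 2–4 second period randomized once at BeginPlay, blinks ElectricBulb off and on with a 2D flicker sound.
; ChangePortrait toggles Girl and Ghost visibility while the light is out, hiding the swap.
; A random branch sometimes adds a second blink, flipping the portrait back.
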(event `self.ReceiveBeginPlay`
  (`KismetSystemLibrary.K2_SetTimerDelegate` (delegate `Light_Sparkle`) (`KismetMathLibrary.RandomFloatInRange` 2.0 4.0) true))

(event `Light_Sparkle`
  (bind _electric_bulb (`self.electric bulb`))
  (`GameplayStatics.PlaySound2D` "/Game/Resouces/Sound/SFX/MainMenu/Light_Flicking_Cue.Light_Flicking_Cue" 1.0 1.0 0.0 null null)
  (`LightComponent.SetIntensity` _electric_bulb 0.0)
  (`KismetSystemLibrary.Delay` 0.1)
  (`self.ChangePortrait`)
  (`LightComponent.SetIntensity` _electric_bulb 1000.0)
  (if (`KismetMathLibrary.RandomBool`)
    (`KismetSystemLibrary.Delay` 0.1)
    (`GameplayStatics.PlaySound2D` "/Game/Resouces/Sound/SFX/MainMenu/Light_Flicking_Cue.Light_Flicking_Cue" 1.0 1.0 0.0 null null)
    (`LightComponent.SetIntensity` _electric_bulb 0.0)
    (`KismetSystemLibrary.Delay` 0.1)
    (`self.ChangePortrait`)
    (`LightComponent.SetIntensity` _electric_bulb 1000.0)))

(fn `ChangePortrait`
  (if (`SceneComponent.bVisible` (`self.Girl`))
    (`SceneComponent.SetVisibility` (`self.Girl`) false false)
    (`SceneComponent.SetVisibility` (`self.Ghost`) true false)
    (else
      (`SceneComponent.SetVisibility` (`self.Ghost`) false false)
      (`SceneComponent.SetVisibility` (`self.Girl`) true false))))

(fn `UserConstructionScript`)