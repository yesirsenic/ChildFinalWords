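; BP_Monster is a ghost enemy that chases the player, damaging them and destroying itself when its AttackBox touches their capsule.
; A timeline bobs the Ghost component and, through a delay, issues AIMoveTo toward the player.
; Tick turns it to face the player and sets walk speed by state.
; Staying beyond TrackingDistance for several seconds escalates Tracking to FastMove, closing in restores Move, and Damaged halts movement.
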(event `self.ReceiveBeginPlay`
  (bind (_direction _moveupdowncomp) (`Timeline|MoveUpDown`)
    (:`Update`
      (`SceneComponent.K2_SetRelativeLocation` (`self.Ghost`) (`KismetMathLibrary.MakeVector` 0.0 0.0 _moveupdowncomp) false false)
      (`KismetSystemLibrary.Delay` 0.4)
      (`|AIMoveTo` self (0.0 0.0 0.0) (`GameplayStatics.GetPlayerCharacter` 0)))))

(event `self.ReceiveTick`
  (params (DeltaSeconds :type "Float (single-precision)"))
  (`self.Follow Rotation`)
  (`self.SetMoveSpeed`)
  (if (not (`|EnumEquality` (`self.MonsterCurrentState`) "Damaged"))
    (`self.SetTrackingState`)
    (`self.SetMoveState` DeltaSeconds)))

(event `self.AttackBox.OnComponentBeginOverlap`
  (params (OverlappedComponent :type "PrimitiveComponent Object Reference") (OtherActor :type "Actor Object Reference") (OtherComp :type "PrimitiveComponent Object Reference") (OtherBodyIndex :type Integer) (bFromSweep :type Boolean) (SweepResult :type "HitResult Structure (by ref)"))
  (bind _asbp_player (cast `/Game/BluePrints/Pure/BP_Player` OtherActor))
  (if (== (`Character.CapsuleComponent` _asbp_player) OtherComp)
    (`/Game/BluePrints/Pure/BP_Player.DamagedByMonster` _asbp_player)
    (`self.K2_DestroyActor`)))

(fn `Follow Rotation`
  (bind _returnvalue (`GameplayStatics.GetPlayerCharacter` 0))
  (bind (_returnvalue_roll _returnvalue_pitch _returnvalue_yaw) (`KismetMathLibrary.BreakRotator` (`KismetMathLibrary.FindLookAtRotation` (`self.K2_GetActorLocation` self) (`self.K2_GetActorLocation` _returnvalue))))
  (if (`KismetSystemLibrary.IsValid` _returnvalue)
    (`self.K2_SetActorRotation` (`KismetMathLibrary.MakeRotator` _returnvalue_roll 0.0 _returnvalue_yaw))))

(fn `SetMoveSpeed`
  (bind _charactermovement (`self.CharacterMovement`))
  (switch `MonsterState` (`self.MonsterCurrentState`)
    (:`Idle`
      (set `CharacterMovementComponent.MaxWalkSpeed` 200.0 _charactermovement))
    (:`Move`
      (set `CharacterMovementComponent.MaxWalkSpeed` 200.0 _charactermovement))
    (:`Damaged`
      (set `CharacterMovementComponent.MaxWalkSpeed` 0.0 _charactermovement))
    (:`Tracking`
      (set `CharacterMovementComponent.MaxWalkSpeed` 200.0 _charactermovement))
    (:`FastMove`
      (set `CharacterMovementComponent.MaxWalkSpeed` 400.0 _charactermovement))))

(fn `SetMoveState`
  (params (DeltaSecond :type "Float (double-precision)"))
  (if (`|EnumEquality` (`self.MonsterCurrentState`) "Tracking")
    (set `self.TrackingTime` (+ DeltaSecond (`self.TrackingTime`)))
    (if (> (`self.TrackingTime`) 5.0)
      (`self.SetState` "FastMove"))
    (else
      (set `self.TrackingTime` 0.0))))

(fn `SetTrackingState`
  (bind _returnvalue (`GameplayStatics.GetPlayerPawn` 0))
  (if (`KismetSystemLibrary.IsValid` _returnvalue)
    (if (> (`KismetMathLibrary.Vector_Distance` (`self.K2_GetActorLocation` self) (`self.K2_GetActorLocation` _returnvalue)) (`self.TrackingDistance`))
      (if (not (`|EnumEquality` (`self.MonsterCurrentState`) "FastMove"))
        (`self.SetState` "Tracking"))
      (else
        (`self.SetState` "Move")))))

(fn `UserConstructionScript`)